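; Mordhau component that forces the controlled character to carry only a Blunderbuss alongside fists.
; Once the match starts, Tick sets up a one-second looping timer, cleared on EndPlay, that calls a server event relaying to a multicast validate.
; Validation caches the Controller's living character; when it changes, all non-fist equipment is dropped and destroyed, then a Blunderbuss is spawned, picked up and equipped.
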(event `self.ReceiveEndPlay`
  (params (EndPlayReason :type "EEndPlayReason Enum" :default "Destroyed"))
  (`KismetSystemLibrary.K2_ClearAndInvalidateTimerHandle` (`self.NewVar_0`))
  (`parent.ReceiveEndPlay` EndPlayReason))

(event `self.ReceiveTick`
  (params (DeltaSeconds :type "Float (single-precision)"))
  (if (`GameStateBase.HasMatchStarted` (`GameplayStatics.GetGameState`))
    (`/Engine/EditorBlueprintResources/StandardMacros.DoOnce` false
      (:`Completed`
        (bind _returnvalue (`KismetSystemLibrary.K2_SetTimerDelegate` (delegate `Server_Validate`) 1.0 true))
        (set `self.NewVar_0` _returnvalue)))))

(event `Server_Validate`
  (`self.Multicast_Validate`))

(event `Multicast_Validate`
  (bind _returnvalue (`self.SetCharacter`))
  (if _returnvalue
    (`self.SpawnBlunderbuss`)))

(fn `SetCharacter`
  (returns (ReturnValue :type Boolean))
  (bind _controller (`self.Controller`))
  (bind _returnvalue (`MordhauPlayerController.GetControlledMordhauCharacter` _controller true))
  (`KismetSystemLibrary.PrintString` "SetCharacter")
  (`/Engine/EditorBlueprintResources/StandardMacros.IsValid` _controller
    (:`Is Valid`
      (`/Engine/EditorBlueprintResources/StandardMacros.IsValid` _returnvalue
        (:`Is Valid`
          (if (`AdvancedCharacter.GetIsDead` _returnvalue)
            (set `self.Character` null :!label _label)
            (elif (== (`self.Character`) _returnvalue)
              _
              (else
                (set `self.Character` _returnvalue)
                (return true)))))
        (:`Is Not Valid`
          (goto _label))))
    (:`Is Not Valid`
      (goto _label)))
  (return false))

(fn `SpawnBlunderbuss`
  (bind _character (`self.Character`))
  (for _array_element (`MordhauCharacter.Equipment` _character)
    (`/Engine/EditorBlueprintResources/StandardMacros.IsValid` _array_element
      (:`Is Valid`
        (cast `/Game/Mordhau/Blueprints/Equipment/Weapons/BP_FistsWeapon` _array_element
          (:`CastFailed`
            (bind _returnvalue (`MordhauCharacter.DropEquipment` _character _array_element true))
            (`Actor.K2_DestroyActor` _returnvalue)
            (`Actor.K2_DestroyActor` _array_element))))))
  (bind _returnvalue_2 (`|SpawnActorFromClass` "/Game/Mordhau/Blueprints/Equipment/Ranged/BP_Blunderbuss.BP_Blunderbuss_C" (`KismetMathLibrary.Conv_VectorToTransform` (`Actor.K2_GetActorLocation` _character)) "Undefined" "OverrideRootScale" null _character))
  (`MordhauCharacter.PickUp` _character _returnvalue_2 -1)
  (`MordhauCharacter.SwitchEquipment` _character _returnvalue_2))