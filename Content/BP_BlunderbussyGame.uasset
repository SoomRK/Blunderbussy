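; Mordhau game-side actor that gives players the Blunderbussy component, except in Horde mode or on maps disabled through config.
; On BeginPlay it destroys itself if the game mode is Horde or a "DisableOnMap" entry in the Blunderbussy config section contains the current level name.
; Otherwise it binds to the Mordhau game mode's after-login event, adding the component to each joining player controller and storing that controller on it.
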(event `self.ReceiveBeginPlay`
  (bind _returnvalue (`GameplayStatics.GetGameMode`))
  (bind _returnvalue_2 (`self.GetConfig`))
  (if _returnvalue_2
    (`self.K2_DestroyActor` :!label _label)
    (else
      (cast `/Game/Mordhau/Blueprints/GameModes/Horde/BP_HordeGameMode` _returnvalue
        (:`then`
          (goto _label))
        (:`CastFailed`
          (bind _asbp_mordhau_game_mode (cast `/Game/Mordhau/Blueprints/GameModes/BP_MordhauGameMode` _returnvalue))
          (add `MordhauGameMode.OnAfterLogin` _asbp_mordhau_game_mode (delegate `OnAfterLogin`)))))))

(event `OnAfterLogin`
  (params (NewPlayer :type "PlayerController Object Reference"))
  (`/Engine/EditorBlueprintResources/StandardMacros.IsValid` NewPlayer
    (:`Is Valid`
      (bind _asbp_mordhau_player_controller (cast `/Game/Mordhau/Blueprints/BP_MordhauPlayerController` NewPlayer))
      (bind _returnvalue (`AddComponent|NODE_AddBP_BlunderbussyComponent-0` :`self` _asbp_mordhau_player_controller))
      (set `/Blunderbussy/BP_BlunderbussyComponent.Controller` _asbp_mordhau_player_controller _returnvalue))))

(fn `GetConfig`
  (returns (ReturnValue :type Boolean))
  (bind (_arraysize _returnvalue) (`MordhauUtilityLibrary.GetCustomConfigVar_Array` "Blunderbussy" "DisableOnMap"))
  (if (> _arraysize 0)
    (bind _returnvalue_2 (`GameplayStatics.GetCurrentLevelName` false))
    (set `self.NewVar_0` _returnvalue_2)
    (for _array_element _returnvalue
      (if (`KismetStringLibrary.Contains` _array_element (`self.NewVar_0`))
        (return true)))
    (else
      (return false))))

(fn `UserConstructionScript`
  (`parent.UserConstructionScript`))